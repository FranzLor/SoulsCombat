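; BP_BaseWeapon is a base weapon actor that registers itself with its owning character's combat setup when equipped.
; OnEquipped extends the parent logic by fetching the owner's BP_CombatComponent, attaching to the hand or stowed socket depending on whether combat is enabled, and setting itself as main weapon.
; It then passes its combat type to the character mesh's anim instance through an UpdateCombatType message.
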(event EventBeginPlay
  (|CallParentFunction) ; This node is disabled and will not be called.\nDrag off pins to build functionality.
)

(event Collision|EventActorBeginOverlap
  (params (OtherActor :type Actor%20Object%20Reference))
  (|CallParentFunction OtherActor) ; This node is disabled and will not be called.\nDrag off pins to build functionality.
)

(event EventTick
  (params (DeltaSeconds :type Float%20%28single-precision%29))
  (|CallParentFunction DeltaSeconds) ; This node is disabled and will not be called.\nDrag off pins to build functionality.
)

(fn ConstructionScript
  (|CallParentFunction))

(fn OnEquipped
  (|CallParentFunction)
  (Variables|Default|SetCombatComponent (Actor|GetComponentbyClass (Components|GetOwner) "/Game/Dynamic/CombatSystem/Blueprints/Components/BP_CombatComponent.BP_CombatComponent_C"))
  (CallFunction|AttachActor (select (Default|IsCombatEnabled (Variables|Default|GetCombatComponent)) (Variables|Initialization|GetHandSocketName) (Variables|Default|GetAttachSocketName)))
  (Default|SetMainWeapon (Variables|Default|GetCombatComponent) self)
  (Class|AnimInstanceBPI|UpdateCombatType(Message) (Components|SkeletalMesh|GetAnimInstance (Variables|/Script/Engine.Character|GetMesh (.AsCharacter (Utilities|Casting|CastToCharacter (Components|GetOwner))))) (Variables|Initialization|GetCombatType)))